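; Interactive window Blueprint that swings a left and a right pane open and closed when Q is pressed.
; Overlapping Window_trigger enables player input, prints a prompt and shows QWindow; leaving disables input and hides it.
; A FlipFlop alternates playing and reversing the Window_func timeline, which drives mirrored yaw on the panes.
; Each toggle plays its own sound at the world origin rather than at the window.
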(event `self.window_trigger.OnComponentBeginOverlap`
  (params (OverlappedComponent :type "PrimitiveComponent Object Reference") (OtherActor :type "Actor Object Reference") (OtherComp :type "PrimitiveComponent Object Reference") (OtherBodyIndex :type Integer) (bFromSweep :type Boolean) (SweepResult :type "HitResult Structure (by ref)"))
  (`KismetSystemLibrary.PrintString` "entry, press q")
  (`self.EnableInput` (`GameplayStatics.GetPlayerController` 0))
  (`SceneComponent.SetVisibility` (`self.q_window`) true false))

(event `self.window_trigger.OnComponentEndOverlap`
  (params (OverlappedComponent :type "PrimitiveComponent Object Reference") (OtherActor :type "Actor Object Reference") (OtherComp :type "PrimitiveComponent Object Reference") (OtherBodyIndex :type Integer))
  (`self.DisableInput` (`GameplayStatics.GetPlayerController` 0))
  (`SceneComponent.SetVisibility` (`self.q_window`) false false))

(event `Key|Q`
  (params (Key :type "Key Structure"))
  (:`Pressed`
    (`/Engine/EditorBlueprintResources/StandardMacros.FlipFlop`
      (:`A`
        (`GameplayStatics.PlaySoundAtLocation` "/Game/foc/audio/mixkit-creaky-door-open-195.mixkit-creaky-door-open-195" (0.0 0.0 0.0) (struct) 1.0 1.0 0.0 null null null null)
        (bind (_direction _window_func_time) (`Timeline|window_func` :!label _label)
          (:`Update`
            (`SceneComponent.K2_SetRelativeRotation` (`self.right_window_pane`) (`KismetMathLibrary.MakeRotator` 0.0 0.0 (* _window_func_time -1.0)) false false)
            (`SceneComponent.K2_SetRelativeRotation` (`self.left_window_pane`) (`KismetMathLibrary.MakeRotator` 0.0 0.0 _window_func_time) false false))))
      (:`B`
        (`GameplayStatics.PlaySoundAtLocation` "/Game/StarterContent/Audio/Collapse_Cue.Collapse_Cue" (0.0 0.0 0.0) (struct) 1.0 1.0 0.0 null null null null)
        (goto _label :!via `Reverse`)))))

(fn `UserConstructionScript`)